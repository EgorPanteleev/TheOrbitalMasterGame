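; Default player controller that creates the main menu overlay and custom mouse pointer, and routes camera input to the player's spaceship.
; ToggleOverlayMode switches between game-and-UI input with cursor and menu shown, and game-only input with both hidden.
; Tick caches the possessed BP_Spaceship, whose camera follows the camera axes when the overlay is off or left mouse is held.
; A mouse-to-world line trace is present but never runs.
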(event `self.ReceiveBeginPlay`
  (bind _returnvalue (`|CreateWidget` "/Game/game/gui/WG_MousePointer.WG_MousePointer_C"))
  (`self.SetMouseCursorWidget` "Default" _returnvalue)
  (bind _returnvalue_2 (`|CreateWidget` "/Game/game/gui/WG_MainMenu.WG_MainMenu_C" self))
  (bind _output_get (set `self.main gui` _returnvalue_2))
  (`UserWidget.AddToViewport` _output_get 0)
  (`self.Toggle overlay Mode`))

(event `Key|Tab`
  (params (Key :type "Key Structure")))

(event `InputAxis|camera_y`
  (params (AxisValue :type "Float (single-precision)"))
  (bind _spaceship (`self.IfSpaceship` :!label _label))
  (`/Game/game/blueprints/BP_Spaceship.Rotate camera by inputs` _spaceship (.x (* (* (`KismetMathLibrary.MakeVector` (`self.GetInputAxisValue`) (`self.GetInputAxisValue`)) (`KismetMathLibrary.Conv_BoolToDouble` (or (`self.View Rotate`) (not (`self.Overlay Enabled`))))) (`KismetMathLibrary.Conv_DoubleToVector` 1.0))) (* (.y (* (* (`KismetMathLibrary.MakeVector` (`self.GetInputAxisValue`) (`self.GetInputAxisValue`)) (`KismetMathLibrary.Conv_BoolToDouble` (or (`self.View Rotate`) (not (`self.Overlay Enabled`))))) (`KismetMathLibrary.Conv_DoubleToVector` 1.0))) -1.0)))

(event `InputAxis|camera_x`
  (params (AxisValue :type "Float (single-precision)"))
  (goto _label))

(event `self.ReceiveTick`
  (params (DeltaSeconds :type "Float (single-precision)"))
  (`|ExecutionSequence`
    (:`then_0`
      (bind _asbp_spaceship (cast `/Game/game/blueprints/BP_Spaceship` (`self.K2_GetPawn`)))
      (set `self.Spaceship` _asbp_spaceship))))

(event `Key|LeftMouseButton`
  (params (Key :type "Key Structure"))
  (:`Pressed`
    (set `self.View Rotate` true))
  (:`Released`
    (set `self.View Rotate` false)))

(event `Key|RightMouseButton`
  (params (Key :type "Key Structure")))

(fn `Set no overlay mode`
  (`WidgetBlueprintLibrary.SetInputMode_GameOnly` self)
  (set `self.bShowMouseCursor` false)
  (`Widget.SetVisibility` (`self.main gui`) "Hidden")
  (return))

(fn `Set overlay mode`
  (`WidgetBlueprintLibrary.SetInputMode_GameAndUIEx` self (`self.main gui`) "DoNotLock" false)
  (set `self.bShowMouseCursor` true)
  (`Widget.SetVisibility` (`self.main gui`) "Visible")
  (return))

(fn `Toggle overlay Mode`
  (bind _overlay_enabled (`self.Overlay Enabled`))
  (if _overlay_enabled
    (`self.Set no overlay mode`)
    (else
      (`self.Set overlay mode`)))
  (set `self.Overlay Enabled` (not _overlay_enabled)))

(fn `UserConstructionScript`)