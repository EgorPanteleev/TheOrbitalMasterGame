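; BP_Trace is a spline mesh segment that forms a straight trace between two given positions.
; The construction script sets both start and end scale to zero, collapsing the mesh's cross-section.
; SetPoints places both ends and uses the unit direction between them as both tangents, deferring the mesh update to the last call.
; Nothing in this graph restores the scale.
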(fn `setPoints`
  (params (StartPos :type "Vector Structure") (EndPos :type "Vector Structure"))
  (bind _returnvalue (`KismetMathLibrary.GetDirectionUnitVector` StartPos EndPos))
  (bind _splinemesh (`self.SplineMesh`))
  (`|ExecutionSequence`
    (:`then_0`
      (`SplineMeshComponent.SetStartPosition` _splinemesh StartPos false))
    (:`then_1`
      (`SplineMeshComponent.SetEndPosition` _splinemesh EndPos false))
    (:`then_2`
      (`SplineMeshComponent.SetStartTangent` _splinemesh _returnvalue false))
    (:`then_3`
      (`SplineMeshComponent.SetEndTangent` _splinemesh _returnvalue true))
    (:`then_4`
      (return))))

(fn `UserConstructionScript`
  (bind _returnvalue (`KismetMathLibrary.Conv_DoubleToVector2D` 0.0))
  (bind _splinemesh (`self.SplineMesh`))
  (`SplineMeshComponent.SetStartScale` _splinemesh _returnvalue true)
  (`SplineMeshComponent.SetEndScale` _splinemesh _returnvalue true))