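; Thruster actor that holds a force vector for an outside caller to clear, accumulate, clamp and read; it applies no force itself.
; Clamping caps magnitude at MaxAcceleration, restricting non-dynamic thrusters to their up axis, with a separate function limiting deviation from a given direction.
; UpdateVisuals aligns dynamic thrusters to the force and spawns physics-driven smoke actors that inherit parent velocity, shrink with age and are culled by lifetime and count.
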(fn `Accamulate Force`
  (params (`Increment value` :type "Vector Structure"))
  (returns (Force :type "Vector Structure"))
  (bind _output_get (set `self.forse` (+ (`self.forse`) `Increment value`)))
  (return _output_get))

(fn `Can Create Smoke Particle`
  (returns (`Can Create` :type Boolean))
  (return (> (`KismetMathLibrary.VSizeSquared` (`self.forse`)) 0.5)))

(fn `Clamp Foce Angle`
  (params (`Default Directory` :type "Vector Structure"))
  (returns (Force :type "Vector Structure"))
  (bind _forse (`self.forse`))
  (bind _returnvalue (`KismetMathLibrary.Cross_VectorVector` `Default Directory` (`KismetMathLibrary.Normal` (`self.forse`))))
  (bind _returnvalue_2 (`KismetMathLibrary.RotateAngleAxis` `Default Directory` (`KismetMathLibrary.FClamp` (`KismetMathLibrary.DegAsin` (`KismetMathLibrary.VSize` _returnvalue)) 0.0 (`self.max angle`)) _returnvalue))
  (bind _output_get (set `self.forse` (* _returnvalue_2 (`KismetMathLibrary.FClamp` (`KismetMathLibrary.Dot_VectorVector` _returnvalue_2 _forse) 0.0 (`KismetMathLibrary.VSize` _forse)))))
  (return _output_get))

(fn `Clamp Force`
  (returns (Force :type "Vector Structure"))
  (bind _returnvalue (`self.GetActorUpVector`))
  (bind _forse (`self.forse`))
  (bind _returnvalue_2 (`KismetMathLibrary.VSize` _forse))
  (bind _returnvalue_3 (* _returnvalue (`KismetMathLibrary.FClamp` (`KismetMathLibrary.Dot_VectorVector` _returnvalue (`self.forse`)) 0.0 100000000.0)))
  (bind _returnvalue_4 (`KismetMathLibrary.VSize` _returnvalue_3))
  (if (`self.dynamic`)
    (bind _output_get (set `self.forse` (* _forse (/ (`KismetMathLibrary.FClamp` _returnvalue_2 0.0 (`self.max acceleration`)) _returnvalue_2))))
    (else
      (set `self.forse` (* _returnvalue_3 (/ (`KismetMathLibrary.FClamp` _returnvalue_4 0.0 (`self.max acceleration`)) _returnvalue_4)))))
  (return _output_get))

(fn `Clear Force`
  (set `self.forse` (0.0 0.0 0.0))
  (return))

(fn `Create Smoke Particle`
  (params (`Parent Velocity` :type "Vector Structure"))
  (bind _returnvalue (`|SpawnActorFromClass` "/Game/game/blueprints/BP_SmokeParticle.BP_SmokeParticle_C" (`KismetMathLibrary.MakeTransform` (.location (`self.GetTransform`)) (.rotation (`self.GetTransform`))) "AlwaysSpawn" "OverrideRootScale" null null))
  (`KismetArrayLibrary.Array_Add` (`self.smoke particles`) _returnvalue)
  (bind _staticmesh (`/Game/game/blueprints/BP_SmokeParticle.StaticMesh` _returnvalue))
  (`PrimitiveComponent.SetMassOverrideInKg` _staticmesh "None" 0.5 true)
  (`PrimitiveComponent.SetPhysicsLinearVelocity` _staticmesh (+ `Parent Velocity` (* (`self.forse`) (* (`self.velocity factor`) 0.05))) false "None")
  (bind _output_get (set `/Game/game/blueprints/BP_SmokeParticle.InitialScale` (* (`KismetMathLibrary.Conv_DoubleToVector` (* (`KismetMathLibrary.RandomFloatInRange` 0.1 1.0) (`self.smoke scale`))) (`KismetMathLibrary.Conv_DoubleToVector` 7.0)) _returnvalue))
  (`SceneComponent.SetWorldScale3D` (`/Game/game/blueprints/BP_SmokeParticle.StaticMesh` _returnvalue) _output_get))

(fn `Get Force`
  (returns (forse :type "Vector Structure"))
  (return (`self.forse`)))

(fn `Update Smoke Particles`
  (params (`Parent Velocity` :type "Vector Structure"))
  (locals (NewLocalVar :type Integer))
  (bind _smoke_particles (`self.smoke particles`))
  (`|ExecutionSequence`
    (:`then_0`
      (for (_array_element _array_index) (`self.smoke particles`)
        (if (> (`self.GetGameTimeSinceCreation` _array_element) (`self.lifetime`))
          (`self.K2_DestroyActor` _array_element)
          (`KismetArrayLibrary.Array_Remove` (`self.smoke particles`) _array_index))))
    (:`then_1`
      (bind _can_create (`self.Can Create Smoke Particle`))
      (if _can_create
        (`self.Create Smoke Particle` `Parent Velocity`)))
    (:`then_2`
      (while (> (`KismetArrayLibrary.Array_Length` (`self.smoke particles`)) (`self.max smoke particles`))
        (`self.K2_DestroyActor` (`|GetArrayItem` _smoke_particles))
        (`KismetArrayLibrary.Array_Remove` _smoke_particles)))
    (:`then_3`
      (for _array_element_2 (`self.smoke particles`)
        (`SceneComponent.SetWorldScale3D` (`/Game/game/blueprints/BP_SmokeParticle.StaticMesh` _array_element_2) (* (`/Game/game/blueprints/BP_SmokeParticle.InitialScale` _array_element_2) (- 1.0 (/ (`self.GetGameTimeSinceCreation` _array_element_2) (`self.lifetime`)))))))))

(fn `Update Visuals`
  (params (`Parent Velocity` :type "Vector Structure"))
  (`|ExecutionSequence`
    (:`then_0`
      (if (`self.dynamic`)
        (`self.K2_SetActorRotation` (`KismetMathLibrary.MakeRotFromZ` (`self.forse`)) true)))
    (:`then_1`
      (`self.Update Smoke Particles` `Parent Velocity`))))

(fn `UserConstructionScript`)