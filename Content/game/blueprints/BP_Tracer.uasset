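; BP_Tracer draws a fading-width trail behind itself as it moves, built from a chain of spawned BP_Trace spline-mesh segments.
; Each Tick it removes segments older than Duration, adds one when CanCreateNewTrace allows, and trims the oldest beyond MaxNumberOfTraces.
; The newest segment's end follows the actor, while every segment's scale shrinks linearly with age.
; DrawTraces toggles segment visibility.
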(event `self.ReceiveTick`
  (params (DeltaSeconds :type "Float (single-precision)"))
  (`|ExecutionSequence`
    (:`then_0`
      (`self.remove timeouted`))
    (:`then_1`
      (`self.update count`))
    (:`then_2`
      (`self.update last point`))
    (:`then_3`
      (`self.update scale`))
    (:`then_4`
      (`self.set visibility`))))

(fn `UserConstructionScript`
  (set `self.prev trace location` (`self.K2_GetActorLocation`)))