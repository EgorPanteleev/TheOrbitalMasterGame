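; Player-controlled physics spaceship that flies under the summed inverse-square gravity of all BP_Planet actors.
; Axis inputs accumulate force on child BP_Thruster actors, which each tick clamp it and apply it at their location; a Calibrate input adds damping.
; The spring-arm camera toggles between ship-relative and independent axis-based rotation, switching to independent during fast spins or far zoom.
; Far zoom also shows a simplified marker and swaps tracer trails.
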(fn `calc gravity`
  (returns (Gravity :type "Vector Structure"))
  (bind _outactors (`GameplayStatics.GetAllActorsOfClass` "/Game/game/blueprints/BP_Planet.BP_Planet_C"))
  (set `self.gravity` (0.0 0.0 0.0))
  (for _array_element _outactors
    (bind _returnvalue (- (`self.K2_GetActorLocation` _array_element) (`self.K2_GetActorLocation`)))
    (set `self.gravity` (+ (* (`KismetMathLibrary.Normal` _returnvalue) (/ (* 1.0 (`/Game/game/blueprints/BP_Planet.mass` _array_element)) (`KismetMathLibrary.MultiplyMultiply_FloatFloat` (/ (`KismetMathLibrary.VSize` _returnvalue) (`self.gravity scale`)) 2.0))) (`self.gravity`))))
  (return (`self.Gravity`)))

(fn `camera x rotate`
  (params (B :type "Float (double-precision)"))
  (bind _camera_independent_rotator (`self.camera independent rotator`))
  (bind _returnvalue (`KismetMathLibrary.GetUpVector` _camera_independent_rotator))
  (bind _returnvalue_2 (`KismetMathLibrary.RotateAngleAxis` (`KismetMathLibrary.GetForwardVector` _camera_independent_rotator) B _returnvalue))
  (bind _output_get (set `self.camera independent rotator` (`KismetMathLibrary.MakeRotationFromAxes` _returnvalue_2 (`KismetMathLibrary.Cross_VectorVector` _returnvalue _returnvalue_2) _returnvalue)))
  (`SceneComponent.K2_SetWorldRotation` (`self.SpringArm`) _output_get false true))

(fn `camera x rotate relative`
  (params (B :type "Float (double-precision)") (Rotation :type "Rotator Structure"))
  (`SceneComponent.K2_SetRelativeRotation` (`self.SpringArm`) (`KismetMathLibrary.MakeRotator` (.roll Rotation) (.pitch Rotation) (+ (.yaw Rotation) B)) false false))

(fn `camera y rotate `
  (params (B :type "Float (double-precision)"))
  (bind _camera_independent_rotator (`self.camera independent rotator`))
  (bind _returnvalue (`KismetMathLibrary.GetUpVector` _camera_independent_rotator))
  (bind _returnvalue_2 (`KismetMathLibrary.GetRightVector` _camera_independent_rotator))
  (bind _output_get (set `self.camera independent rotator` (`KismetMathLibrary.MakeRotationFromAxes` (`KismetMathLibrary.Cross_VectorVector` _returnvalue_2 (`KismetMathLibrary.RotateAngleAxis` _returnvalue (* B -1.0) _returnvalue_2)) _returnvalue_2 _returnvalue)))
  (`SceneComponent.K2_SetWorldRotation` (`self.SpringArm`) _output_get false true))

(fn `camera y rotate relative`
  (params (B :type "Float (double-precision)") (Rotation :type "Rotator Structure"))
  (`SceneComponent.K2_SetRelativeRotation` (`self.SpringArm`) (`KismetMathLibrary.MakeRotator` (.roll Rotation) (`KismetMathLibrary.FClamp` (+ (.pitch Rotation) B) -80.0 80.0) (.yaw Rotation)) false false))

(fn `camera z rotate`
  (params (AngleDeg :type "Float (single-precision)"))
  (bind _camera_independent_rotator (`self.camera independent rotator`))
  (bind _returnvalue (`KismetMathLibrary.GetForwardVector` _camera_independent_rotator))
  (bind _returnvalue_2 (`KismetMathLibrary.RotateAngleAxis` (`KismetMathLibrary.GetRightVector` _camera_independent_rotator) AngleDeg _returnvalue))
  (bind _output_get (set `self.camera independent rotator` (`KismetMathLibrary.MakeRotationFromAxes` _returnvalue _returnvalue_2 (`KismetMathLibrary.Cross_VectorVector` _returnvalue _returnvalue_2))))
  (`SceneComponent.K2_SetWorldRotation` (`self.SpringArm`) _output_get false true))

(fn `Fire All In Direction`
  (params (right :type "Float (double-precision)") (back :type "Float (double-precision)") (left :type "Float (double-precision)") (direction :type "Vector Structure (by ref)")))

(fn `fire jet`
  (params (thrust :type "ChildActorComponent Object Reference") (Forse :type "Vector Structure") (InDouble :type "Float (double-precision)"))
  (bind _asbp_thruster (cast `/Game/game/blueprints/BP_Thruster` (`ChildActorComponent.ChildActor` thrust)))
  (`/Game/game/blueprints/BP_Thruster.Accamulate Force` _asbp_thruster (* Forse (`KismetMathLibrary.Conv_DoubleToVector` (* InDouble 10000.0))))
  (return))

(fn `get_current planet`)

(fn `Rotate camera by inputs`
  (params (x1 :type "Float (double-precision)") (y1 :type "Float (double-precision)"))
  (locals (x :type "Float (double-precision)") (y :type "Float (double-precision)"))
  (bind _returnvalue (`self.camera aligned`))
  (switch `int` (`self.camera type`)
    (:`0`
      (`|ExecutionSequence`
        (:`then_0`
          (`self.camera x rotate relative` x1 _returnvalue))
        (:`then_1`
          (`self.camera y rotate relative` y1 _returnvalue)))
      (set `self.camera independent rotator` (`SceneComponent.K2_GetComponentRotation` (`self.SpringArm`))))
    (:`1`
      (`self.Rotate camera independent` x1 y1))))

(fn `Rotate camera independent`
  (params (x1 :type "Float (double-precision)") (y1 :type "Float (double-precision)"))
  (`|ExecutionSequence`
    (:`then_0`
      (`self.camera y rotate ` y1))
    (:`then_1`
      (if (`self.camera_rotate_z`)
        (`self.camera z rotate` x1)
        (else
          (`self.camera x rotate` x1))))))

(fn `set speed`
  (params (power :type "Float (double-precision)"))
  (bind _asbp_thruster (cast `/Game/game/blueprints/BP_Thruster` (`ChildActorComponent.ChildActor` (`self.forward`))))
  (set `/Game/game/blueprints/BP_Thruster.power` (* power 10.0) _asbp_thruster)
  (return))

(fn `Update Thrusters`
  (locals (Thruster :type "/Game/game/blueprints/BP_Thruster Object Reference"))
  (bind _asthrust (`self.for thrust`)
    (:`then`
      (set `local.Thruster` _asthrust)
      (`|ExecutionSequence`
        (:`then_0`
          (`/Game/game/blueprints/BP_Thruster.Clamp Force` (`local.Thruster`)))
        (:`then_1`
          (bind _forse (`/Game/game/blueprints/BP_Thruster.Get Force` (`local.Thruster`)))
          (`PrimitiveComponent.AddForceAtLocation` (`self.StaticMesh`) (`KismetMathLibrary.NegateVector` _forse) (`SceneComponent.K2_GetComponentLocation` (`/Game/game/blueprints/BP_Thruster.StaticMesh` (`local.Thruster`))) "None"))
        (:`then_2`
          (bind _returnvalue (`PrimitiveComponent.GetPhysicsLinearVelocity` (`self.StaticMesh`) "None"))
          (`/Game/game/blueprints/BP_Thruster.Update Visuals` (`local.Thruster`) _returnvalue))
        (:`then_3`
          (`/Game/game/blueprints/BP_Thruster.Clear Force` (`local.Thruster`)))))))

(fn `UserConstructionScript`)